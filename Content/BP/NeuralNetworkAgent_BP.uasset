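; Reinforcement learning agent pawn that bridges the game to a Python neural network through a TensorflowComponent.
; It begins training on play, sends game state and network data as JSON custom function calls, and ends the session on EndPlay.
; Python events drive the loop: state requests trigger takeAction, reset events reset the game mode, and step events pass the chosen action to the agent.
; Older JSON input and result handlers remain disconnected.
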(event OnInputResults(TensorflowComponent)
  (params (Results :type String))
  ;[1 1 1] Send next inputs to agent from neural network after 'onJsonInput' (unused)
)

(event OnTrainingComplete(TensorflowComponent)
  (params (SummaryJson :type String))
  ;[1 1 1] On Training Complete() (unused)
)

(event OnEvent(TensorflowComponent)
  (params (Event :type String) (Data :type String))
  ;[1 1 1] Python Call Events
  (Utilities|FlowControl|Sequence
    (:then_0
      (if (Utilities|Enum|Equal(Enum) Event "GetStateEvent")
        (bind _returnvalue (Class|NeuralNetworkAgent|GetState))
        (Class|NeuralNetworkAgent|SetOldState _returnvalue)
        (Default|CallCustomFunction (Variables|Default|GetTensorflowComponent) "takeAction" (Class|SIOJsonObject|EncodeJson (Class|SIOJLibrary|StructtoJsonObject _returnvalue)))))
    (:then_1
      (if (Utilities|Enum|Equal(Enum) Event "ResetGameEvent")
        (bind _asreinforcement_game_game_mode (Utilities|Casting|CastToReinforcementGameGameMode (Game|GetGameMode)))
        (Class|ReinforcementGameGameMode|ResetGame _asreinforcement_game_game_mode)))
    (:then_2
      (if (Utilities|Enum|Equal(Enum) Event "TakeAStepEvent")
        (Class|NeuralNetworkAgent|OnTakeAStepEvent (Class|SIOJLibrary|ToInteger(JsonValue) (Class|SIOJsonObject|GetField (Class|SIOJLibrary|ToJsonObject(JsonValue) (Class|SIOJsonValue|ValuefromJsonString Data)) "action")))))))

(event EventBeginPlay
  ;[1 1 1] Begin Training
  (Default|BeginTraining (Variables|Default|GetTensorflowComponent)))

(event Collision|EventActorBeginOverlap
  (params (OtherActor :type Actor%20Object%20Reference)))

(event EventTick
  (params (DeltaSeconds :type Float%20%28single-precision%29)))

(event EventSendGameStatetoNeuralNetwork
  ;[1 1 1] Send State to Network (onJsonInput) (unused)
)

(event EventSendNetworkData
  (params (NetworkData :type HOTRELOADED%20Network%20Data%20Struct%200%20Structure))
  ;[1 1 1] Send All Current Data To Network
  (bind _returnvalue (Class|SIOJsonObject|ConstructJsonObject))
  (Class|SIOJsonObject|SetObjectField _returnvalue "data" (Class|SIOJLibrary|StructtoJsonObject NetworkData))
  (Default|CallCustomFunction (Variables|Default|GetTensorflowComponent) "sendNetworkData" (Class|SIOJsonObject|EncodeJson _returnvalue)))

(event EventStartNeuralNetwork
  ;[1 1 1] Start Neural Network
  (Default|CallCustomFunction (Variables|Default|GetTensorflowComponent) "start" "_"))

(event EventInitMaterialandColor
  (bind _returnvalue (Class|Agent|GetMesh))
  ;[1 1 1] Init Material And Color
  (Utilities|IsValid _returnvalue
    (:Is%20Valid
      (bind _returnvalue_2 (Rendering|Material|CreateDynamicMaterialInstance _returnvalue 0 "/Game/StarterContent/Materials/M_Basic_Floor.M_Basic_Floor" "None" :!class /Script/Engine.PrimitiveComponent))
      (Rendering|Material|SetVectorParameterValue _returnvalue_2 "Color" (Variables|Default|GetAgentColor) :!class /Script/Engine.MaterialInstanceDynamic))))

(event EventEndPlay
  (params (EndPlayReason :type EEndPlayReason%20Enum :default "Destroyed"))
  (bind _tensorflowcomponent (Variables|Default|GetTensorflowComponent))
  ;[1 1 1] EndPlay()
  (Default|StopTraining _tensorflowcomponent)
  (Default|CallCustomFunction _tensorflowcomponent "endSession"))

(fn ConstructionScript)